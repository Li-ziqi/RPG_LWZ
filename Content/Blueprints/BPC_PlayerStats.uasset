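; Player stats component for BP_ThirdPersonCharacter that tracks health and endurance and mirrors them on the character's HUD bars.
; It caches the owning character one tick after BeginPlay.
; Decrease functions return true once a stat is depleted, while increase functions clamp to the maximum.
; Health and endurance changes push percentages straight to the HUD, except raising max endurance, which leaves the bar unchanged.
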(event `self.ReceiveBeginPlay`
  (`KismetSystemLibrary.DelayUntilNextTick`)
  (bind _asbp_third_person_character (cast `/Game/ThirdPerson/Blueprints/BP_ThirdPersonCharacter` (`self.GetOwner`)))
  (set `self.As BP Third Person Character` _asbp_third_person_character))

(fn `Decrease Endurance`
  (params (`Endurance Health` :type "Float (double-precision)"))
  (returns (`is Consumed` :type Boolean))
  (bind _endurance (`self.Endurance`))
  (if (not (<= _endurance 0.0))
    (bind _output_get (set `self.Endurance` (- _endurance `Endurance Health`)))
    (`ProgressBar.SetPercent` (`/Game/UI/WP_HUD.Endurance` (`/Game/ThirdPerson/Blueprints/BP_ThirdPersonCharacter.HUD` (`self.As BP Third Person Character`))) (/ _output_get (`self.MaxEndurance`)))
    (if (<= _output_get 0.0)
      _
      (else
        (return false))))
  (return true))

(fn `Decrease Health`
  (params (Damage :type "Float (double-precision)"))
  (returns (`is death` :type Boolean))
  (if (not (<= (`self.Health`) 0.0))
    (bind _output_get (set `self.Health` (- (`self.Health`) Damage)))
    (`ProgressBar.SetPercent` (`/Game/UI/WP_HUD.Health` (`/Game/ThirdPerson/Blueprints/BP_ThirdPersonCharacter.HUD` (`self.As BP Third Person Character`))) (/ _output_get (`self.MaxHealth`)))
    (if (<= _output_get 0.0)
      _
      (else
        (return false))))
  (return true))

(fn `Increase Endurance`
  (params (`Add Endurance` :type "Float (double-precision)"))
  (bind _maxendurance (`self.MaxEndurance`))
  (bind _output_get (set `self.Endurance` (+ (`self.Endurance`) `Add Endurance`)))
  (if (> _output_get _maxendurance)
    (bind _output_get_2 (set `self.Endurance` _maxendurance)))
  (if (not (<= _output_get_2 0.0))
    (`ProgressBar.SetPercent` (`/Game/UI/WP_HUD.Endurance` (`/Game/ThirdPerson/Blueprints/BP_ThirdPersonCharacter.HUD` (`self.As BP Third Person Character`))) (/ _output_get_2 (`self.MaxEndurance`)))))

(fn `Increase Health`
  (params (`add Health` :type "Float (double-precision)"))
  (bind _maxhealth (`self.MaxHealth`))
  (bind _output_get (set `self.Health` (+ (`self.Health`) `add Health`)))
  (if (> _output_get _maxhealth)
    (bind _output_get_2 (set `self.Health` _maxhealth)))
  (`ProgressBar.SetPercent` (`/Game/UI/WP_HUD.Health` (`/Game/ThirdPerson/Blueprints/BP_ThirdPersonCharacter.HUD` (`self.As BP Third Person Character`))) (/ _output_get_2 (`self.MaxHealth`))))

(fn `Increase Max Endurance`
  (params (B :type "Float (double-precision)"))
  (set `self.MaxEndurance` (+ (`self.MaxEndurance`) B)))

(fn `Increase Max Health`
  (params (`Add Health` :type "Float (double-precision)"))
  (set `self.MaxHealth` (+ (`self.MaxHealth`) `Add Health`))
  (`ProgressBar.SetPercent` (`/Game/UI/WP_HUD.Health` (`/Game/ThirdPerson/Blueprints/BP_ThirdPersonCharacter.HUD` (`self.As BP Third Person Character`))) (/ (`self.Health`) (`self.MaxHealth`))))