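; BP_Dummy is a stealth-kill target that the player can assassinate from behind.
; An Assassination overlap shows or hides a prompt widget for BP_ThirdPersonCharacter, and Tick turns that widget toward the camera.
; StealthBackAssasin plays the paired knife victim montage, hides the prompt, triggers a delayed mesh ragdoll, and returns the AssasinREF location and actor rotation to the caller.
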(event `self.ReceiveTick`
  (params (DeltaSeconds :type "Float (single-precision)"))
  (bind _assassinationwidget (`self.AssassinationWidget`))
  (`SceneComponent.K2_SetWorldRotation` _assassinationwidget (`KismetMathLibrary.FindLookAtRotation` (`SceneComponent.K2_GetComponentLocation` _assassinationwidget) (`SceneComponent.K2_GetComponentLocation` (`Actor.RootComponent` (`GameplayStatics.GetPlayerCameraManager` 0)))) false false))

(event `Ragdoll`
  (`KismetSystemLibrary.Delay` 2.5)
  (`PrimitiveComponent.SetSimulatePhysics` (`self.Mesh`) true))

(event `self.Assassination.OnComponentBeginOverlap`
  (params (OverlappedComponent :type "PrimitiveComponent Object Reference") (OtherActor :type "Actor Object Reference") (OtherComp :type "PrimitiveComponent Object Reference") (OtherBodyIndex :type Integer) (bFromSweep :type Boolean) (SweepResult :type "HitResult Structure (by ref)"))
  (cast `/Game/ThirdPerson/Blueprints/BP_ThirdPersonCharacter` OtherActor)
  (`SceneComponent.SetVisibility` (`self.AssassinationWidget`) true false))

(event `self.Assassination.OnComponentEndOverlap`
  (params (OverlappedComponent :type "PrimitiveComponent Object Reference") (OtherActor :type "Actor Object Reference") (OtherComp :type "PrimitiveComponent Object Reference") (OtherBodyIndex :type Integer))
  (cast `/Game/ThirdPerson/Blueprints/BP_ThirdPersonCharacter` OtherActor)
  (`SceneComponent.SetVisibility` (`self.AssassinationWidget`) false false))

(fn `Stealth Back Assasin`
  (returns (`位置` :type "Vector Structure") (`旋转` :type "Rotator Structure"))
  (`self.PlayAnimMontage` "/Game/Characters/Animations/Assassination/Paired_Knife_Stealth_KidneyAndNeck_Vic1_Montage.Paired_Knife_Stealth_KidneyAndNeck_Vic1_Montage")
  (`self.Ragdoll`)
  (`SceneComponent.SetVisibility` (`self.AssassinationWidget`) false false)
  (return (`SceneComponent.K2_GetComponentLocation` (`self.Assasin REF`)) (`self.K2_GetActorRotation`)))

(fn `UserConstructionScript`)